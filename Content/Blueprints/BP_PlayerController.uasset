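; Player controller for a multiplayer dice game, handling dice rolls, lobby UI, chat, kicking and the escape menu.
; Hero rolls spawn one D6 at a random tagged spawner and monster rolls one at every tagged spawner, each launched downward with random rotation.
; Chat messages fan out through the GameMode's controller list into each UI_main chat window and are saved to GameMode history.
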(event `self.ReceiveBeginPlay`)

(event `HeroDiceRoll`
  ;[1 1 1] Hero Dice Roll
  (`KismetSystemLibrary.PrintString` "Hero Dice Rolled")
  (bind _outactors (`GameplayStatics.GetAllActorsWithTag` "HeroSpawner"))
  (bind _returnvalue (`|SpawnActorFromClass` "/Game/Blueprints/D6Hero.D6Hero_C" (`KismetMathLibrary.MakeTransform` (`self.K2_GetActorLocation` (`|GetArrayItem` _outactors (`KismetMathLibrary.RandomIntegerInRange` 0 (`self.DiceNumber`)))) (`KismetMathLibrary.RandomRotator` true)) "AdjustIfPossibleButAlwaysSpawn" "OverrideRootScale" null null))
  (`PrimitiveComponent.SetAllPhysicsLinearVelocity` (`StaticMeshActor.StaticMeshComponent` _returnvalue) (0.0 0.0 -3500.0) true))

(event `MonsterDiceRoll`
  ;[1 1 1] Monster Dice Roll
  (`KismetSystemLibrary.PrintString` "Monster Dice Rolled")
  (bind _outactors (`GameplayStatics.GetAllActorsWithTag` "MonsterSpawner"))
  (for _array_element _outactors
    (bind _returnvalue (`|SpawnActorFromClass` "/Game/Blueprints/D6Monster.D6Monster_C" (`KismetMathLibrary.MakeTransform` (`self.K2_GetActorLocation` _array_element) (`KismetMathLibrary.RandomRotator` true)) "AdjustIfPossibleButAlwaysSpawn" "OverrideRootScale" null null))
    (`PrimitiveComponent.SetAllPhysicsLinearVelocity` (`StaticMeshActor.StaticMeshComponent` _returnvalue) (0.0 0.0 -3500.0) true)))

(event `ClearDice`
  ;[1 1 1] Clear Dice
  (bind _outactors (`GameplayStatics.GetAllActorsOfClass` "/Game/Blueprints/D6Hero.D6Hero_C"))
  (`self.K2_DestroyActor` _outactors)
  (bind _outactors_2 (`GameplayStatics.GetAllActorsOfClass` "/Game/Blueprints/D6Monster.D6Monster_C"))
  (`self.K2_DestroyActor` _outactors_2))

(event `Key|Escape`
  (params (Key :type "Key Structure"))
  ;[1 1 1] Escape Menu
  (:`Pressed`
    (`WidgetLayoutLibrary.RemoveAllWidgets`)
    (bind _returnvalue (`|CreateWidget` "/Game/Blueprints/UI/Escape_menu.Escape_menu_C" (`GameplayStatics.GetPlayerController` 0)))
    (`UserWidget.AddToViewport` _returnvalue 0)))

(event `AddMessageFromServerToEachPlayer`
  (params (Message :type String) (Color :type "SlateColor Structure") (`isServerMessage?` :type Boolean))
  (bind _chatmessagestructure (make `/Game/Blueprints/ChatMessageStructure` (`AdvancedSessionsLibrary.GetPlayerName` self) Message Color `isServerMessage?`))
  ;[1 1 1] Chat System
  (bind _asnew_game_mode (cast `/Game/Blueprints/UI/NewGameMOde` (`GameplayStatics.GetGameMode`)))
  (for _array_element (`/Game/Blueprints/UI/NewGameMOde.AllPCs` _asnew_game_mode)
    (bind _asbp_player_controller (cast `/Game/Blueprints/BP_PlayerController` _array_element))
    (`self.AddMessageToChat` _asbp_player_controller _chatmessagestructure))
  (bind _asnew_game_mode_2 (cast `/Game/Blueprints/UI/NewGameMOde` (`GameplayStatics.GetGameMode`)))
  (`/Game/Blueprints/UI/NewGameMOde.AddMessageToChatHistory` _asnew_game_mode_2 _chatmessagestructure))

(event `AddMessageToChat`
  (params (ChatMessage :type "/Game/Blueprints/ChatMessageStructure Structure"))
  ;[1 1 1] Chat System
  (`/Game/Blueprints/UI/ChatWindow.AddChildToChat` (`/Game/Blueprints/UI/UI_main.ChatWindow` (`self.UI_main`)) ChatMessage))

(event `ClearPlayerList`
  (`/Game/Blueprints/UI/UI_main.ClearPlayerList` (`self.UI_main`)))

(event `AddLobbyWB`
  (bind _returnvalue (`|CreateWidget` "/Game/Blueprints/UI/UI_main.UI_main_C" (`GameplayStatics.GetPlayerController` 0)))
  (bind _output_get (set `self.UI_main` _returnvalue))
  (`UserWidget.AddToViewport` _output_get 1))

(event `Kick`
  (params (KickIndex :type Integer))
  (`GameplayStatics.OpenLevel` "Menu")
  (`DestroySessionCallbackProxy.DestroySession` self))

(event `LoadingScreen`
  (`Widget.RemoveFromParent` (`self.UI_main`))
  (bind _returnvalue (`|CreateWidget` "/Game/Blueprints/UI/LoadingScreen.LoadingScreen_C" self))
  (`UserWidget.AddToViewport` _returnvalue 0))

(event `AddPlayer`
  (params (`Fail?` :type Boolean) (Player :type Text) (Avatar :type "Texture2D Object Reference") (PlayerIndex :type Integer))
  (`/Game/Blueprints/UI/UI_main.AddPlayerToList` (`self.UI_main`) `Fail?` Player Avatar PlayerIndex))

(fn `UserConstructionScript`)