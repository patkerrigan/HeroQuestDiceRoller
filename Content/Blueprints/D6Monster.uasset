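; D6Monster is a six-sided die actor that tracks which of its faces points up.
; Each Tick loops over FacesNormals, rotates each normal by the actor transform and dots it with world up.
; The first normal past a fixed threshold stores its one-based index in UpFace and breaks the loop; UpFace stays zero when no face qualifies.
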(event `self.ReceiveTick`
  (params (DeltaSeconds :type "Float (single-precision)"))
  (for (_array_element _array_index) (`self.Faces Normals`) :!label _label
    (set `self.Up Face` 0)
    (if (> (`KismetMathLibrary.Dot_VectorVector` (`KismetMathLibrary.TransformDirection` (`self.GetTransform`) _array_element) (0.0 0.0 1.0)) 0.6)
      (set `self.Up Face` (+ _array_index 1))
      (`self.Break ForEachLoop`))))

(event `Break ForEachLoop`
  (goto _label :!via `Break`))

(fn `UserConstructionScript`)